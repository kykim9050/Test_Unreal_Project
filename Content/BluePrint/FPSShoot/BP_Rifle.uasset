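; BP_Rifle is a pickup rifle for an FPS, with firing that so far only traces and reports what it hits.
; PickUpComponent's OnPickUp event passes the character to WeaponComponent, which attaches the weapon to it.
; While WeaponComponent's IsFire is set, Tick runs a Visibility line trace forward from that component every frame, drawing a debug line and printing the hit actor's name without applying damage.
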(event OnPickUp(PickUpComponent)
  (params (PickUpCharacter :type FPS%20Character%20Object%20Reference))
  (Class|FPSWeaponComponent|AttachWeapon (Variables|Default|GetWeaponComponent) PickUpCharacter))

(event EventTick
  (params (DeltaSeconds :type Float%20%28single-precision%29))
  (bind _weaponcomponent (Variables|Default|GetWeaponComponent))
  (bind _returnvalue (Transformation|GetWorldLocation _weaponcomponent))
  (if (Variables|/Script/PracticePJ.FPS_WeaponComponent|GetIsFire _weaponcomponent)
    (bind _outhit (Collision|LineTraceByChannel _returnvalue (+ _returnvalue (* (Math|Vector|GetForwardVector (Transformation|GetWorldRotation _weaponcomponent)) 3e+03)) "TraceTypeQuery1" false 0 "ForOneFrame"))
    (Development|PrintString (Utilities|GetDisplayName (.HitActor (Collision|BreakHitResult _outhit))))))

(event Collision|EventActorBeginOverlap
  (params (OtherActor :type Actor%20Object%20Reference)))

(event EventBeginPlay)

(fn ConstructionScript)