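; BP_Weapon is a pickup weapon for an FPS that attaches to the character who picks it up.
; PickUpComponent's OnPickUp passes that character to ItemComponent's AttachWeapon.
; While ItemComponent's IsFire is set, Tick runs a Visibility line trace forward from that component every frame.
; The trace is debug-drawn and only prints the hit actor's name, with no damage applied.
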(event OnPickUp(PickUpComponent)
  (params (PickUpCharacter :type FPS%20Character%20Object%20Reference))
  (Class|FPSItemComponent|AttachWeapon (Variables|Default|GetItemComponent) PickUpCharacter))

(event EventTick
  (params (DeltaSeconds :type Float%20%28single-precision%29))
  (bind _itemcomponent (Variables|Default|GetItemComponent))
  (bind _returnvalue (Transformation|GetWorldLocation _itemcomponent))
  (if (Variables|/Script/PracticePJ.FPS_ItemComponent|GetIsFire _itemcomponent)
    (bind _outhit (Collision|LineTraceByChannel _returnvalue (+ _returnvalue (* (Math|Vector|GetForwardVector (Transformation|GetWorldRotation _itemcomponent)) 3e+03)) "TraceTypeQuery1" false 0 "ForOneFrame"))
    (Development|PrintString (Utilities|GetDisplayName (.HitActor (Collision|BreakHitResult _outhit))))))

(event Collision|EventActorBeginOverlap
  (params (OtherActor :type Actor%20Object%20Reference)))

(event EventBeginPlay)

(fn ConstructionScript)